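; Targeting component that picks and stores a lock-on actor for its owning Character, printing whether a valid target was found.
; A sphere trace around the character gathers actors implementing BPI_TargetingInterface.
; Each gets a camera-to-actor visibility trace; those with a hit are scored by the dot product of camera forward and character-to-target direction.
; Scores are compared to CompareTarget, which is only reassigned to itself, and FindClosestTarget returns no explicit value.
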(event `self.ReceiveBeginPlay`
  (bind _ascharacter (cast `Character` (`self.GetOwner`)))
  (set `self.Character Ref` _ascharacter)
  (set `self.Camera Ref` (`Actor.GetComponentByClass` (`self.Character Ref`) "/Script/Engine.CameraComponent")))

(event `Lock  On To Target`
  (bind _outclosesttarget (`self.Find Closest Target` (`self.Find Actors To Lock On To`)))
  (`/Engine/EditorBlueprintResources/StandardMacros.IsValid` _outclosesttarget
    (:`Is Valid`
      (set `self.Locked On Actor` _outclosesttarget)
      (`KismetSystemLibrary.PrintString` "Valid Target"))
    (:`Is Not Valid`
      (`KismetSystemLibrary.PrintString` "Not Valid Target"))))

(fn `Check How Close Target Is`
  (params (Target :type "Actor Object Reference"))
  (returns (ReturnValue :type "Float (double-precision)"))
  (return (`KismetMathLibrary.Dot_VectorVector` (`SceneComponent.GetForwardVector` (`self.Camera Ref`)) (`KismetMathLibrary.Conv_RotatorToVector` (`KismetMathLibrary.FindLookAtRotation` (`Actor.K2_GetActorLocation` (`self.Character Ref`)) (`Actor.K2_GetActorLocation` Target))))))

(fn `Find Actors To Lock On To`
  (returns (TargetingActors :type "Array of Actor Object Reference"))
  (locals (PotentialTargetingActors :type "Array of Actor Object Reference"))
  (bind _returnvalue (`Actor.K2_GetActorLocation` (`self.Character Ref`)))
  (bind (_outhits _returnvalue_2) (`KismetSystemLibrary.SphereTraceMultiForObjects` _returnvalue _returnvalue (`self.Radius`) (`|MakeArray` "ObjectTypeQuery7" :!type "EObjectTypeQuery Enum") false (`|MakeArray` (`self.GetOwner`))))
  (for _array_element _outhits
    (bind (_bblockinghit _binitialoverlap _time _distance _location _impactpoint _normal _impactnormal _physmat _hitactor) (`GameplayStatics.BreakHitResult` _array_element))
    (if (and _returnvalue_2 (`KismetSystemLibrary.DoesImplementInterface` _hitactor "/Game/Targeting/BPI_TargetingInterface.BPI_TargetingInterface_C"))
      (`KismetArrayLibrary.Array_Add` (`local.PotentialTargetingActors`) _hitactor)))
  (return (`local.PotentialTargetingActors`)))

(fn `Find Closest Target`
  (params (Actors :type "Array of Actor Object Reference"))
  (returns (OutClosestTarget :type "Actor Object Reference"))
  (locals (CompareTarget :type "Float (double-precision)") (ClosestTarget :type "Actor Object Reference"))
  (bind _comparetarget (`local.CompareTarget`))
  (for _array_element Actors
    (bind (_outhit _returnvalue) (`KismetSystemLibrary.LineTraceSingle` :`Start` (`SceneComponent.K2_GetComponentLocation` (`self.Camera Ref`)) :`End` (`Actor.K2_GetActorLocation` _array_element) :`TraceChannel` "TraceTypeQuery1" :`DrawDebugType` "ForDuration"))
    (if _returnvalue
      (`/Engine/EditorBlueprintResources/StandardMacros.CompareFloat` (`self.Check How Close Target Is` _array_element) _comparetarget
        (:`>`
          (set `local.CompareTarget` _comparetarget)
          (set `local.ClosestTarget` _array_element)))))
  (return null))